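; BP_Tile is a board tile actor in a multiplayer chess template, showing its number through a text render.
; BeginPlay writes TileNumber to the text, while TileNumbers forwards a number to TileNumbersSvr, which stores it without refreshing the text.
; The chess functions for availability, move checks, tile lookup, mode and piece movement are stubs returning empty or default values.
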(event `self.ReceiveBeginPlay`
  (`TextRenderComponent.K2_SetText` (`self.TextRender`) (`KismetTextLibrary.Conv_IntToText` (`self.TileNumber`))))

(event `/Game/MPChessTemplate/Blueprints/BPI_ChessInterface.TileNumbers`
  (params (Number :type Integer))
  (`self.TileNumbersSvr` Number))

(event `TileNumbersSvr`
  (params (TileNumber :type Integer))
  (set `self.TileNumber` TileNumber))

(fn `CheckAvailable`
  (params (Tiles :type "Array of /Game/MPChessTemplate/Blueprints/BP_Tile Object Reference (by ref)"))
  (returns (OpenTiles :type "Array of Integer"))
  (return))

(fn `CheckPieceMoves`
  (returns (ValidMoves :type "Array of Integer") (CheckTIles :type "Array of Integer") (`InCheck?` :type Boolean) (KingTile :type "/Game/MPChessTemplate/Blueprints/BP_Tile Object Reference") (AttackingPieces :type "Array of /Game/MPChessTemplate/Blueprints/BP_ChessPieces Object Reference"))
  (return _ _ false null))

(fn `FindTileByIndex`
  (params (Index :type Integer))
  (returns (Tile :type "/Game/MPChessTemplate/Blueprints/BP_Tile Object Reference"))
  (return null))

(fn `GetMode`
  (returns (Mode :type Integer))
  (return 0))

(fn `MovePiece`
  (params (Piece :type "/Game/MPChessTemplate/Blueprints/BP_ChessPieces Object Reference") (Tile :type "/Game/MPChessTemplate/Blueprints/BP_Tile Object Reference") (Number :type Integer) (Location :type "Vector Structure"))
  (returns (`Success?` :type Boolean))
  (return false))

(fn `UserConstructionScript`)