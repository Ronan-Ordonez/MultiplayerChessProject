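; BP_DamageAmount is an actor that shows a floating damage number and then removes itself.
; On BeginPlay it passes its DamageAmount to the WBP_DamageNumber widget in its widget component.
; A Move timeline then lerps the actor from its spawn location to a raised, slightly offset point, and destroys it when finished.
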(event `self.ReceiveBeginPlay`
  (bind _aswbp_damage_number (cast `/Game/MPChessTemplate/UI/WBP_DamageNumber` (`WidgetComponent.GetWidget` (`self.Widget`))))
  (`/Game/MPChessTemplate/UI/WBP_DamageNumber.SetAmount` _aswbp_damage_number (`self.DamageAmount`))
  (bind _output_get (set `self.StartLoc` (`self.K2_GetActorLocation`)))
  (set `self.EndLoc` (+ _output_get (-25.0 -25.0 100.0)))
  (bind (_direction _movetrack) (`Timeline|Move`)
    (:`Update`
      (`self.K2_SetActorLocation` (`KismetMathLibrary.VLerp` (`self.StartLoc`) (`self.EndLoc`) _movetrack)))
    (:`Finished`
      (`self.K2_DestroyActor`))))

(fn `UserConstructionScript`)