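; Base chess piece for a chess game with Fire Emblem-style combat, with placeholder move-validation and check functions.
; MovePiece validates moves, then captures outright or, depending on game mode, starts combat with counterattacks and speed-based follow-ups.
; Combat uses stats rolled from data-table growth rates, weapon data and crits, spawning damage-number actors.
; It also reports king check to the game state and plays a timeline-driven camera-and-leap attack cutscene.
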(event `PlayCutscene`
  (bind (_zoomendrotation_roll _zoomendrotation_pitch _zoomendrotation_yaw) (`KismetMathLibrary.BreakRotator` (`self.ZoomEndRotation`)))
  (bind (_leapendrotation_roll _leapendrotation_pitch _leapendrotation_yaw) (`KismetMathLibrary.BreakRotator` (`self.LeapEndRotation`)))
  (bind (_returnvalue_roll _returnvalue_pitch _returnvalue_yaw) (`KismetMathLibrary.BreakRotator` (`self.K2_GetActorRotation` self)))
  (bind (_returnvalue_roll_2 _returnvalue_pitch_2 _returnvalue_yaw_2) (`KismetMathLibrary.BreakRotator` (`SceneComponent.K2_GetComponentRotation` (`/Game/MPChessTemplate/Blueprints/BP_CameraPawn.SpringArm` (`self.CameraPawn`)))))
  (`KismetSystemLibrary.PrintString` (`KismetSystemLibrary.GetDisplayName` self) true true (struct :`G` 0.66 :`B` 1.0 :`A` 1.0) 100.0)
  (bind (_direction _zoomprogress) (`Timeline|Zoom` :!via `PlayFromStart`)
    (:`Update`
      (`SceneComponent.K2_SetWorldLocationAndRotation` (`/Game/MPChessTemplate/Blueprints/BP_CameraPawn.SpringArm` (`self.CameraPawn`)) (`KismetMathLibrary.VLerp` (`SceneComponent.K2_GetComponentLocation` (`/Game/MPChessTemplate/Blueprints/BP_CameraPawn.SpringArm` (`self.CameraPawn`))) (`SceneComponent.K2_GetComponentLocation` (`self.SpringArm`)) _zoomprogress) (`KismetMathLibrary.RLerp` (`SceneComponent.K2_GetComponentRotation` (`/Game/MPChessTemplate/Blueprints/BP_CameraPawn.SpringArm` (`self.CameraPawn`))) (`SceneComponent.K2_GetComponentRotation` (`self.SpringArm`)) _zoomprogress) false false))
    (:`Finished`
      (set `self.RotateEndPosition` (+ (`SceneComponent.K2_GetComponentLocation` (`/Game/MPChessTemplate/Blueprints/BP_CameraPawn.SpringArm` (`self.CameraPawn`))) (`self.ZoomEndPosition`)))
      (set `self.RotateEndRotation` (`KismetMathLibrary.MakeRotator` (+ _returnvalue_roll_2 _zoomendrotation_roll) (+ _zoomendrotation_pitch _returnvalue_pitch_2) (+ _zoomendrotation_yaw _returnvalue_yaw_2)))
      (bind (_direction_2 _progress) (`Timeline|Attack` :!via `PlayFromStart`)
        (:`Update`
          (`SceneComponent.K2_SetWorldLocationAndRotation` (`/Game/MPChessTemplate/Blueprints/BP_CameraPawn.SpringArm` (`self.CameraPawn`)) (`KismetMathLibrary.VLerp` (`SceneComponent.K2_GetComponentLocation` (`/Game/MPChessTemplate/Blueprints/BP_CameraPawn.SpringArm` (`self.CameraPawn`))) (`self.RotateEndPosition`) _progress) (`KismetMathLibrary.RLerp` (`SceneComponent.K2_GetComponentRotation` (`/Game/MPChessTemplate/Blueprints/BP_CameraPawn.SpringArm` (`self.CameraPawn`))) (`self.RotateEndRotation`) _progress) false false))
        (:`Finished`
          (set `self.LeapEndPosition_0` (+ (`self.K2_GetActorLocation` self) (`self.LeapEndPosition`)))
          (set `self.LeapEndRotation_0` (`KismetMathLibrary.MakeRotator` (+ _returnvalue_roll _leapendrotation_roll) (+ _returnvalue_pitch _leapendrotation_pitch) (+ _returnvalue_yaw _leapendrotation_yaw)))
          (bind (_direction_3 _leapprogress) (`Timeline|Leap` :!via `PlayFromStart`)
            (:`Update`
              (`self.SvrPieceLeap` self 0 (`KismetMathLibrary.VLerp` (`self.K2_GetActorLocation` self) (`self.LeapEndPosition_0`) _leapprogress) (`KismetMathLibrary.RLerp` (`self.K2_GetActorRotation` self) (`self.LeapEndRotation_0`) _leapprogress) null))))))))

(event `self.ReceiveBeginPlay`
  (`|ExecutionSequence`
    (:`then_0`
      (bind _asbp_chess_game_mode (cast `/Game/MPChessTemplate/Blueprints/BP_ChessGameMode` (`GameplayStatics.GetGameMode`)))
      (set `self.As Chess Game Mode` _asbp_chess_game_mode))
    (:`then_1`
      (`KismetSystemLibrary.Delay` 1.0)
      (bind _outactors (`GameplayStatics.GetAllActorsOfClass` "/Game/MPChessTemplate/Blueprints/BP_Tile.BP_Tile_C"))
      (set `self.Out Actors` _outactors))
    (:`then_2`
      (bind _asbp_chess_game_state (cast `/Game/MPChessTemplate/Blueprints/BP_ChessGameState` (`GameplayStatics.GetGameState`)))
      (set `self.As Chess Game State` _asbp_chess_game_state))
    (:`then_3`
      (`/Engine/EditorBlueprintResources/ActorMacros.Switch Has Authority`
        (:`Authority`
          (`KismetSystemLibrary.Delay` 2.8)
          (`self.KingInCheck?`))))
    (:`then_4`
      (bind _asbp_chess_player_controller (cast `/Game/MPChessTemplate/Blueprints/BP_ChessPlayerController` (`GameplayStatics.GetPlayerController` 0)))
      (set `self.CameraPawn` (`/Game/MPChessTemplate/Blueprints/BP_ChessPlayerController.CameraPawn` _asbp_chess_player_controller)))
    (:`then_5`
      (`self.CalculateStats`))))

(event `SvrPieceLeap`
  (params (Tile :type Integer) (NewLocation :type "Vector Structure") (NewRotation :type "Rotator Structure") (TargetActor :type "/Game/MPChessTemplate/Blueprints/BP_Tile Object Reference"))
  (`SceneComponent.K2_SetWorldLocationAndRotation` (`self.StaticMesh`) NewLocation NewRotation false false))

(event `SvrDamage`
  (params (Attacker :type "/Game/MPChessTemplate/Blueprints/BP_ChessPieces Object Reference") (Defender :type "/Game/MPChessTemplate/Blueprints/BP_ChessPieces Object Reference") (Tile :type "/Game/MPChessTemplate/Blueprints/BP_Tile Object Reference") (TileNum :type Integer) (Location :type "Vector Structure"))
  (bind _defeated_ (`self.InflictDamage` Attacker Defender))
  (if _defeated_
    (bind _mode (message `/Game/MPChessTemplate/Blueprints/BPI_ChessInterface.GetMode` (`GameplayStatics.GetGameMode`) :!label _label))
    (if (< _mode 2)
      (`self.SvrPieceMove` Attacker TileNum Location Tile)
      (`/Game/MPChessTemplate/Blueprints/BP_ChessGameMode.Destroy` (`self.As Chess Game Mode`) Defender)
      (else
        (`self.SvrClearTile` Tile)
        (`/Game/MPChessTemplate/Blueprints/BP_ChessGameMode.Destroy` (`self.As Chess Game Mode`) Defender)))
    (else
      (`KismetSystemLibrary.Delay` 1.6)
      (bind _defeated__2 (`self.InflictDamage` Defender Attacker))
      (if _defeated__2
        (bind _outactors (`GameplayStatics.GetAllActorsOfClass` "/Game/MPChessTemplate/Blueprints/BP_Tile.BP_Tile_C" :!label _label_2))
        (for _array_element _outactors
          (if (== (`/Game/MPChessTemplate/Blueprints/BP_Tile.TileNumber` _array_element) (`/Game/MPChessTemplate/Blueprints/BP_ChessPieces.CurrentTile` Attacker))
            (`self.SvrClearTile` _array_element)))
        (`/Game/MPChessTemplate/Blueprints/BP_ChessGameMode.Destroy` (`self.As Chess Game Mode`) Attacker)
        (else
          (`KismetSystemLibrary.Delay` 1.6)
          (if (`self.CalcSpeed` Attacker Defender)
            (bind _defeated__3 (`self.InflictDamage` Attacker Defender))
            (if _defeated__3
              (goto _label))
            (elif (`self.CalcSpeed` Defender Attacker)
              (bind _defeated__4 (`self.InflictDamage` Defender Attacker))
              (if _defeated__4
                (goto _label_2)))))))))

(event `SvrPieceMove`
  (params (Tile :type Integer) (NewLocation :type "Vector Structure") (TargetActor :type "/Game/MPChessTemplate/Blueprints/BP_Tile Object Reference"))
  ;[1 1 1] Piece Move Execution
  (bind (_sweephitresult _returnvalue) (`self.K2_SetActorLocation` NewLocation))
  (set `/Game/MPChessTemplate/Blueprints/BP_Tile.Occupied` _returnvalue TargetActor)
  (if _returnvalue
    (set `self.CurrentTile` Tile)
    (set `self.CurrentTileBP` TargetActor)))

(event `/Game/MPChessTemplate/Blueprints/BPI_ChessInterface.DamagePiece`
  (params (Instagator :type "/Game/MPChessTemplate/Blueprints/BP_ChessPieces Object Reference") (Reciever :type "/Game/MPChessTemplate/Blueprints/BP_ChessPieces Object Reference") (Tile :type "/Game/MPChessTemplate/Blueprints/BP_Tile Object Reference") (TileNum :type Integer) (Location :type "Vector Structure"))
  (`self.SvrDamage` Instagator Reciever Tile TileNum Location))

(event `/Game/MPChessTemplate/Blueprints/BPI_ChessInterface.DestroyPiece`
  (params (Piece :type "/Game/MPChessTemplate/Blueprints/BP_ChessPieces Object Reference"))
  ;[1 1 1] Piece Elimanation
  (`self.SvrDestroyPiece` self))

(event `/Game/MPChessTemplate/Blueprints/BPI_ChessInterface.SelectPiece`
  ;[1 1 1] Piece Selection
  (`SceneComponent.SetVisibility` (`self.Decal`) true false))

(event `SvrDestroyPiece`
  (params (Target :type "/Game/MPChessTemplate/Blueprints/BP_ChessPieces Object Reference"))
  (bind _as_chess_game_state (`self.As Chess Game State`))
  ;[1 1 1] Piece Elimanation
  (bind _outactors (`GameplayStatics.GetAllActorsOfClass` "/Game/MPChessTemplate/Blueprints/BP_King.BP_King_C"))
  (for _array_element _outactors
    (`/Game/MPChessTemplate/Blueprints/BPI_ChessInterface.DestroyPiece` _array_element self))
  (`|ExecutionSequence`
    (:`then_0`
      (`/Game/MPChessTemplate/Blueprints/BPI_ChessInterface.DamagePiece` _as_chess_game_state self Target null 0 (0.0 0.0 0.0)))
    (:`then_1`
      (`KismetSystemLibrary.Delay` 0.2)
      (message `/Game/MPChessTemplate/Blueprints/BPI_ChessInterface.CheckAllPieces` _as_chess_game_state null))))

(event `/Game/MPChessTemplate/Blueprints/BPI_ChessInterface.DeselectPiece`
  ;[1 1 1] Piece Selection
  (`SceneComponent.SetVisibility` (`self.Decal`) false false))

(event `SvrClearTile`
  (params (Tile :type "/Game/MPChessTemplate/Blueprints/BP_Tile Object Reference"))
  (`/Engine/EditorBlueprintResources/StandardMacros.IsValid` Tile
    (:`Is Valid`
      (set `/Game/MPChessTemplate/Blueprints/BP_Tile.Piece` null Tile)
      (set `/Game/MPChessTemplate/Blueprints/BP_Tile.Occupied` false Tile))))

(event `KingInCheck?`
  (bind _team (`self.Team`))
  (bind _team_2 (`self.Team`))
  (bind _as_chess_game_state (`self.As Chess Game State`))
  (bind _as_chess_game_state_2 (`self.As Chess Game State`))
  ;[1 1 1] King in-check Regular Testing
  (`KismetArrayLibrary.Array_Clear` (`self.ValidMoves`))
  (bind (_validmoves _checktiles _incheck_ _kingtile) (`/Game/MPChessTemplate/Blueprints/BPI_ChessInterface.CheckPieceMoves`))
  (set `self.ValidMoves` _validmoves)
  (if _incheck_
    (switch `int` _team
      (:`1`
        (`/Game/MPChessTemplate/Blueprints/BPI_ChessInterface.KingCheckRelay` _as_chess_game_state_2 (+ _team 1) true _checktiles _kingtile))
      (:`2`
        (`/Game/MPChessTemplate/Blueprints/BPI_ChessInterface.KingCheckRelay` _as_chess_game_state_2 (- _team 1) true _checktiles _kingtile)))
    (else
      (`KismetArrayLibrary.Array_Clear` (`self.InCheckTiles`))
      (switch `int` _team_2
        (:`1`
          (`/Game/MPChessTemplate/Blueprints/BPI_ChessInterface.KingCheckRelay` _as_chess_game_state (+ _team_2 1) false _checktiles _kingtile))
        (:`2`
          (`/Game/MPChessTemplate/Blueprints/BPI_ChessInterface.KingCheckRelay` _as_chess_game_state (- _team_2 1) false _checktiles _kingtile))))))

(event `CalculateStats`
  (bind _returnvalue (`|GetDataTableRow` "/Game/MPChessTemplate/Blueprints/DT_FireEmblemPieces.DT_FireEmblemPieces" (`self.NameByDT`))
    (:`then`
      (bind (_piece _newname _classgrowthrates _defaultgrowthrates _level _movement) (break `/Game/MPChessTemplate/Blueprints/ST_FireEmblem` _returnvalue))
      (set `self.Movement` _movement)
      (bind (_hp _str _mag _dex _spd _lck _def _res _cha _bld) (break `/Game/MPChessTemplate/Blueprints/ST_Stats` _classgrowthrates))
      (bind (_hp_2 _str_2 _mag_2 _dex_2 _spd_2 _lck_2 _def_2 _res_2 _cha_2 _bld_2) (break `/Game/MPChessTemplate/Blueprints/ST_Stats` _defaultgrowthrates))
      (bind _statnew (`self.RollForStat` _level (+ _hp _hp_2)))
      (bind _statnew_2 (`self.RollForStat` _level (+ _str _str_2)))
      (bind _statnew_3 (`self.RollForStat` _level (+ _mag _mag_2)))
      (bind _statnew_4 (`self.RollForStat` _level (+ _dex _dex_2)))
      (bind _statnew_5 (`self.RollForStat` _level (+ _spd _spd_2)))
      (bind _statnew_6 (`self.RollForStat` _level (+ _lck _lck_2)))
      (bind _statnew_7 (`self.RollForStat` _level (+ _def _def_2)))
      (bind _statnew_8 (`self.RollForStat` _level (+ _res _res_2)))
      (bind _statnew_9 (`self.RollForStat` _level (+ _cha _cha_2)))
      (bind _statnew_10 (`self.RollForStat` _level (+ _bld _bld_2)))
      (bind _output_get (set `self.UnitStats` (make `/Game/MPChessTemplate/Blueprints/ST_Stats` _statnew _statnew_2 _statnew_3 _statnew_4 _statnew_5 _statnew_6 _statnew_7 _statnew_8 _statnew_9 _statnew_10)))
      (set `self.CurrentHP` (break `/Game/MPChessTemplate/Blueprints/ST_Stats` _output_get)))))

(fn `CalcSpeed`
  (params (Attacker :type "/Game/MPChessTemplate/Blueprints/BP_ChessPieces Object Reference") (Defender :type "/Game/MPChessTemplate/Blueprints/BP_ChessPieces Object Reference"))
  (returns (`GoesTwice?` :type Boolean))
  (locals (AS1 :type Integer) (AS2 :type Integer))
  (bind (_unitstats_hp _unitstats_str _unitstats_mag _unitstats_dex _unitstats_spd) (break `/Game/MPChessTemplate/Blueprints/ST_Stats` (`/Game/MPChessTemplate/Blueprints/BP_ChessPieces.UnitStats` Defender)))
  (bind (_unitstats_hp_2 _unitstats_str_2 _unitstats_mag_2 _unitstats_dex_2 _unitstats_spd_2) (break `/Game/MPChessTemplate/Blueprints/ST_Stats` (`/Game/MPChessTemplate/Blueprints/BP_ChessPieces.UnitStats` Attacker)))
  (bind _returnvalue (`|GetDataTableRow` "/Game/MPChessTemplate/Blueprints/DT_Weapons.DT_Weapons" (`|GetArrayItem` (`/Game/MPChessTemplate/Blueprints/BP_ChessPieces.Weapons` Attacker)))
    (:`then`
      (set `local.AS1` (- _unitstats_spd_2 (- (`.Weight_7_9860D7894B8E5BCFC3B6C697CA3EEB99` (break `/Game/MPChessTemplate/Blueprints/ST_Weapon` _returnvalue)) (/ _unitstats_str_2 5))))
      (bind _returnvalue_2 (`|GetDataTableRow` "/Game/MPChessTemplate/Blueprints/DT_Weapons.DT_Weapons" (`|GetArrayItem` (`/Game/MPChessTemplate/Blueprints/BP_ChessPieces.Weapons` Defender)))
        (:`then`
          (set `local.AS2` (- _unitstats_spd (- (`.Weight_7_9860D7894B8E5BCFC3B6C697CA3EEB99` (break `/Game/MPChessTemplate/Blueprints/ST_Weapon` _returnvalue_2)) (/ _unitstats_str 5))))
          (return (> (`local.AS1`) (+ (`local.AS2`) 4))))))))

(fn `CheckAvailable`
  (params (Tiles :type "Array of /Game/MPChessTemplate/Blueprints/BP_Tile Object Reference (by ref)"))
  (returns (OpenTiles :type "Array of Integer"))
  (return))

(fn `CheckPieceMoves`
  (returns (ValidMoves :type "Array of Integer") (CheckTIles :type "Array of Integer") (`InCheck?` :type Boolean) (KingTile :type "/Game/MPChessTemplate/Blueprints/BP_Tile Object Reference") (AttackingPieces :type "Array of /Game/MPChessTemplate/Blueprints/BP_ChessPieces Object Reference"))
  (return _ _ false null))

(fn `EatEnemyPiece`)

(fn `FindTileByIndex`
  (params (Index :type Integer))
  (returns (Tile :type "/Game/MPChessTemplate/Blueprints/BP_Tile Object Reference"))
  (return null))

(fn `GetCritRate`
  (params (Attacker :type "/Game/MPChessTemplate/Blueprints/BP_ChessPieces Object Reference") (Defender :type "/Game/MPChessTemplate/Blueprints/BP_ChessPieces Object Reference"))
  (returns (CritRate :type Integer))
  (bind (_unitstats_hp _unitstats_str _unitstats_mag _unitstats_dex _unitstats_spd _unitstats_lck) (break `/Game/MPChessTemplate/Blueprints/ST_Stats` (`/Game/MPChessTemplate/Blueprints/BP_ChessPieces.UnitStats` Defender)))
  (bind (_unitstats_hp_2 _unitstats_str_2 _unitstats_mag_2 _unitstats_dex_2 _unitstats_spd_2 _unitstats_lck_2) (break `/Game/MPChessTemplate/Blueprints/ST_Stats` (`/Game/MPChessTemplate/Blueprints/BP_ChessPieces.UnitStats` Attacker)))
  (return (- (+ _unitstats_dex_2 (/ _unitstats_lck_2 2)) _unitstats_lck)))

(fn `GetDamge`
  (params (Attacker :type "/Game/MPChessTemplate/Blueprints/BP_ChessPieces Object Reference") (Defender :type "/Game/MPChessTemplate/Blueprints/BP_ChessPieces Object Reference"))
  (returns (Damage :type Integer) (`Crit?` :type Boolean))
  (bind (_unitstats_hp _unitstats_str _unitstats_mag _unitstats_dex _unitstats_spd _unitstats_lck _unitstats_def _unitstats_res) (break `/Game/MPChessTemplate/Blueprints/ST_Stats` (`/Game/MPChessTemplate/Blueprints/BP_ChessPieces.UnitStats` Defender)))
  (bind (_unitstats_hp_2 _unitstats_str_2 _unitstats_mag_2) (break `/Game/MPChessTemplate/Blueprints/ST_Stats` (`/Game/MPChessTemplate/Blueprints/BP_ChessPieces.UnitStats` Attacker)))
  (bind _returnvalue (<= (`KismetMathLibrary.RandomIntegerInRange` 1 100) (`self.GetCritRate` (`local.Attacker`) (`local.Defender`))))
  (bind _returnvalue_2 (`|GetDataTableRow` "/Game/MPChessTemplate/Blueprints/DT_Weapons.DT_Weapons" (`|GetArrayItem` (`/Game/MPChessTemplate/Blueprints/BP_ChessPieces.Weapons` Attacker)))
    (:`then`
      (bind (_name _might _weight _hit _range _physical) (break `/Game/MPChessTemplate/Blueprints/ST_Weapon` _returnvalue_2))
      (if _physical
        (`KismetSystemLibrary.PrintString` "Hello")
        (bind _returnvalue_3 (- (+ _might _unitstats_str_2) _unitstats_def))
        (return (`KismetMathLibrary.SelectInt` (* _returnvalue_3 2) _returnvalue_3 _returnvalue) _returnvalue)
        (else
          (bind _returnvalue_4 (- (+ _might _unitstats_mag_2) _unitstats_res))
          (return (`KismetMathLibrary.SelectInt` (* _returnvalue_4 2) _returnvalue_4 _returnvalue) _returnvalue))))))

(fn `GetMode`
  (returns (Mode :type Integer))
  (return 0))

(fn `InflictDamage`
  (params (Attacker :type "/Game/MPChessTemplate/Blueprints/BP_ChessPieces Object Reference") (Defender :type "/Game/MPChessTemplate/Blueprints/BP_ChessPieces Object Reference"))
  (returns (`Defeated?` :type Boolean))
  (bind (_damage _crit_) (`self.GetDamge` (`local.Attacker`) (`local.Defender`)))
  (bind _returnvalue (`KismetMathLibrary.Clamp` _damage 0 999))
  (`|SpawnActorFromClass` "/Game/MPChessTemplate/Blueprints/BP_DamageAmount.BP_DamageAmount_C" (`self.GetTransform` (`local.Defender`)) "Undefined" "MultiplyWithRoot" null _returnvalue _crit_ null)
  (bind _output_get (set `/Game/MPChessTemplate/Blueprints/BP_ChessPieces.CurrentHP` (- (`/Game/MPChessTemplate/Blueprints/BP_ChessPieces.CurrentHP` (`local.Defender`)) _returnvalue) (`local.Defender`)))
  (return (<= _output_get 0)))

(fn `MovePiece`
  (params (Piece :type "/Game/MPChessTemplate/Blueprints/BP_ChessPieces Object Reference") (Tile :type "/Game/MPChessTemplate/Blueprints/BP_Tile Object Reference") (Number :type Integer) (Location :type "Vector Structure"))
  (returns (`Success?` :type Boolean))
  (bind _occupied (`/Game/MPChessTemplate/Blueprints/BP_Tile.Occupied` Tile))
  (if (== Number (`self.CurrentTile`))
    _
    (elif (not (`/Game/MPChessTemplate/Blueprints/BP_Tile.King?` Tile))
      (for _array_element (`self.Out Actors`)
        (if (== (`self.CurrentTile`) (`/Game/MPChessTemplate/Blueprints/BP_Tile.TileNumber` _array_element))
          (set `/Game/MPChessTemplate/Blueprints/BP_Tile.Piece` null _array_element)
          (set `self.LastTile` _array_element)
          (break)))
      ;[1 1 1] Regular Piece Move Command
      (bind _valid (`self.PieceMoveLogic` Number _occupied (`self.FirstMove?`) (and _occupied (!= (`self.Team`) (`/Game/MPChessTemplate/Blueprints/BP_Tile.Team` Tile))) (`self.KingChecked`)))
      (if _valid
        (if _occupied
          (if (!= (`/Game/MPChessTemplate/Blueprints/BP_Tile.Team` Tile) (`self.Team`))
            (bind _piece (`/Game/MPChessTemplate/Blueprints/BP_Tile.Piece` Tile)
              (:`then`
                (bind _mode (message `/Game/MPChessTemplate/Blueprints/BPI_ChessInterface.GetMode` (`GameplayStatics.GetGameMode`)))
                (if (> _mode 0)
                  (`/Game/MPChessTemplate/Blueprints/BPI_ChessInterface.DamagePiece` _piece self _piece (`local.Tile`) (`local.Number`) (`local.Location`))
                  (return true)
                  (else
                    (`self.SvrPieceMove` Number Location Tile)
                    (`/Game/MPChessTemplate/Blueprints/BP_ChessGameMode.Destroy` (`self.As Chess Game Mode`) _piece))))
              (:`else`
                (`self.SvrPieceMove` Number Location Tile :!label _label)))
            (else
              (return false)))
          (else
            (goto _label)))
        (`|ExecutionSequence`
          (:`then_0`
            (`self.KingInCheck?`)
            (`/Game/MPChessTemplate/Blueprints/BPI_ChessInterface.CheckAllPieces` (`self.As Chess Game State`) self)
            (bind _mode_2 (message `/Game/MPChessTemplate/Blueprints/BPI_ChessInterface.GetMode` (`GameplayStatics.GetGameMode`)))
            (if (< _mode_2 3)
              _))
          (:`then_1`
            (set `self.FirstMove?` false)
            (set `/Game/MPChessTemplate/Blueprints/BP_Tile.Piece` self Tile)
            (set `/Game/MPChessTemplate/Blueprints/BP_Tile.Team` (`self.Team`) Tile)
            (set `/Game/MPChessTemplate/Blueprints/BP_Tile.Occupied` false (`self.LastTile`))
            (return true)))
        (else
          (return false))))))

(fn `PieceMoveLogic`
  (params (Tile :type Integer) (`Occupied?` :type Boolean) (`FirstMove?` :type Boolean) (`EnemyOccupied?` :type Boolean) (`KingInCheck?` :type Boolean))
  (returns (Valid :type Boolean) (Take :type Boolean))
  (return true false))

(fn `RollForStat`
  (params (Level :type Integer) (Stat :type Integer))
  (returns (StatNew :type Integer))
  (locals (L_Stat :type Integer))
  (for _ (range (+ Level 1))
    (if (<= (`KismetMathLibrary.RandomIntegerInRange` 1 100) Stat)
      (bind _result (`/Engine/EditorBlueprintResources/StandardMacros.IncrementInt` (`local.L_Stat`))
        (:`  `
          (set `local.L_Stat` _result)))))
  (return (`local.L_Stat`)))

(fn `SetHasMoved`
  (params (`HasMoved?` :type Boolean))
  (set `self.HasMoved?` `HasMoved?`)
  (`KismetSystemLibrary.PrintString` "This Piece has already moved"))

(fn `UserConstructionScript`)