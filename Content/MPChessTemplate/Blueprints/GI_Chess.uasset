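; GI_Chess holds the current mode for the multiplayer chess template and exposes it through GetMode.
; ROS_SETMDOE forwards a new mode to MCSETMDOE, named as a server-to-multicast pair, which stores it and updates the ModeWidget text on every BP_ChessPlayerController.
; The board functions for tile lookup, availability, check detection and piece movement are empty stubs returning default values.
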(event `ROS_SETMDOE`
  (params (Mode :type Integer))
  (`self.MCSETMDOE` Mode))

(event `MCSETMDOE`
  (params (Mode :type Integer))
  (set `self.Mode` Mode)
  (bind _outactors (`GameplayStatics.GetAllActorsOfClass` "/Game/MPChessTemplate/Blueprints/BP_ChessPlayerController.BP_ChessPlayerController_C"))
  (for _array_element _outactors
    (`/Game/MPChessTemplate/UI/WBP_GameMode.SetText` (`/Game/MPChessTemplate/Blueprints/BP_ChessPlayerController.ModeWidget` _array_element) (`self.Mode`))))

(fn `CheckAvailable`
  (params (Tiles :type "Array of /Game/MPChessTemplate/Blueprints/BP_Tile Object Reference (by ref)"))
  (returns (OpenTiles :type "Array of Integer"))
  (return))

(fn `CheckPieceMoves`
  (returns (ValidMoves :type "Array of Integer") (CheckTIles :type "Array of Integer") (`InCheck?` :type Boolean) (KingTile :type "/Game/MPChessTemplate/Blueprints/BP_Tile Object Reference") (AttackingPieces :type "Array of /Game/MPChessTemplate/Blueprints/BP_ChessPieces Object Reference"))
  (return _ _ false null))

(fn `FindTileByIndex`
  (params (Index :type Integer))
  (returns (Tile :type "/Game/MPChessTemplate/Blueprints/BP_Tile Object Reference"))
  (return null))

(fn `GetMode`
  (returns (Mode :type Integer))
  (return (`self.Mode`)))

(fn `MovePiece`
  (params (Piece :type "/Game/MPChessTemplate/Blueprints/BP_ChessPieces Object Reference") (Tile :type "/Game/MPChessTemplate/Blueprints/BP_Tile Object Reference") (Number :type Integer) (Location :type "Vector Structure"))
  (returns (`Success?` :type Boolean))
  (return false))