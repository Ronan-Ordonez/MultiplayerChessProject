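; BP_BoardManager is a board manager actor for the multiplayer chess template, mostly a skeleton in its current state.
; On BeginPlay it only caches the chess game state.
; Disconnected graphs hold unused logic for building an 8x8 checkered board from index math, as either spawned BP_Tile actors or static mesh components.
; Its move, check, tile-lookup, availability and mode functions are stubs returning empty or default values.
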(event `self.ReceiveBeginPlay`
  (`|ExecutionSequence`
    (:`then_0`
      (bind _asbp_chess_game_state (cast `/Game/MPChessTemplate/Blueprints/BP_ChessGameState` (`GameplayStatics.GetGameState`)))
      (set `self.As Chess Game State` _asbp_chess_game_state))))

(fn `CheckAvailable`
  (params (Tiles :type "Array of /Game/MPChessTemplate/Blueprints/BP_Tile Object Reference (by ref)"))
  (returns (OpenTiles :type "Array of Integer"))
  (return))

(fn `CheckPieceMoves`
  (returns (ValidMoves :type "Array of Integer") (CheckTIles :type "Array of Integer") (`InCheck?` :type Boolean) (KingTile :type "/Game/MPChessTemplate/Blueprints/BP_Tile Object Reference") (AttackingPieces :type "Array of /Game/MPChessTemplate/Blueprints/BP_ChessPieces Object Reference"))
  (return _ _ false null))

(fn `FindTileByIndex`
  (params (Index :type Integer))
  (returns (Tile :type "/Game/MPChessTemplate/Blueprints/BP_Tile Object Reference"))
  (return null))

(fn `GetMode`
  (returns (Mode :type Integer))
  (return 0))

(fn `MovePiece`
  (params (Piece :type "/Game/MPChessTemplate/Blueprints/BP_ChessPieces Object Reference") (Tile :type "/Game/MPChessTemplate/Blueprints/BP_Tile Object Reference") (Number :type Integer) (Location :type "Vector Structure"))
  (returns (`Success?` :type Boolean))
  (return false))

(fn `UserConstructionScript`)