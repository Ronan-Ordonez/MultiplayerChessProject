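; BP_Knight is the knight chess piece, defining its move rules on a 64-tile board indexed by number.
; StepUnit offsets give candidate tiles, filtered by modulo/division tests for the L-shape to prevent edge wrapping.
; PieceMoveLogic validates a requested tile, limited to InCheckTiles when in check; CheckAvailable lists L-shaped candidates.
; CheckPieceMoves scans tile actors for empty or enemy-held destinations, reporting any checked king and the tiles involved.
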(fn `CheckAvailable`
  (params (Tiles :type "Array of /Game/MPChessTemplate/Blueprints/BP_Tile Object Reference (by ref)"))
  (returns (OpenTiles :type "Array of Integer"))
  (locals (LocalTiles :type "Array of Integer"))
  (bind _currenttile (`self.CurrentTile`))
  (bind _localtiles (`local.LocalTiles`))
  (bind _currenttile_2 (`self.CurrentTile`))
  (for _array_element (`self.StepUnit`)
    (`|ExecutionSequence`
      (:`then_0`
        (bind _returnvalue (- _currenttile_2 _array_element))
        (bind _returnvalue_2 (`KismetMathLibrary.Abs_Int` (- (mod _returnvalue 8) (mod _currenttile_2 8))))
        (bind _returnvalue_3 (`KismetMathLibrary.Abs_Int` (- (/ _returnvalue 8) (/ _currenttile_2 8))))
        (if (or (and (== _returnvalue_2 1) (== _returnvalue_3 2)) (and (== _returnvalue_2 2) (== _returnvalue_3 1)))
          (`KismetArrayLibrary.Array_Add` _localtiles _returnvalue)))
      (:`then_1`
        (bind _returnvalue_4 (+ _currenttile _array_element))
        (bind _returnvalue_5 (`KismetMathLibrary.Abs_Int` (- (mod _returnvalue_4 8) (mod _currenttile 8))))
        (bind _returnvalue_6 (`KismetMathLibrary.Abs_Int` (- (/ _returnvalue_4 8) (/ _currenttile 8))))
        (if (or (and (== _returnvalue_5 1) (== _returnvalue_6 2)) (and (== _returnvalue_5 2) (== _returnvalue_6 1)))
          (`KismetArrayLibrary.Array_Add` _localtiles _returnvalue_4)))))
  (return (`local.LocalTiles`)))

(fn `CheckPieceMoves`
  (returns (ValidMoves :type "Array of Integer") (CheckTIles :type "Array of Integer") (`InCheck?` :type Boolean) (KingTile :type "/Game/MPChessTemplate/Blueprints/BP_Tile Object Reference") (AttackingPieces :type "Array of /Game/MPChessTemplate/Blueprints/BP_ChessPieces Object Reference"))
  (locals (`check?` :type Boolean) (Kngtile :type "/Game/MPChessTemplate/Blueprints/BP_Tile Object Reference") (chktiles :type "Array of Integer"))
  (bind _currenttile (`self.CurrentTile`))
  (bind _currenttile_2 (`self.CurrentTile`))
  (bind _validmoves (`self.ValidMoves`))
  (set `local.Kngtile` null)
  (set `local.check?` false)
  (`KismetArrayLibrary.Array_Clear` (`self.ValidMoves`))
  (`KismetArrayLibrary.Array_Clear` (`self.InCheckTiles`))
  (for _array_element (`self.StepUnit`)
    (`|ExecutionSequence`
      (:`then_0`
        (bind _returnvalue (- _currenttile_2 _array_element))
        (bind _returnvalue_2 (`KismetMathLibrary.Abs_Int` (- (mod _returnvalue 8) (mod _currenttile_2 8))))
        (bind _returnvalue_3 (`KismetMathLibrary.Abs_Int` (- (/ _returnvalue 8) (/ _currenttile_2 8))))
        (if (or (and (== _returnvalue_2 1) (== _returnvalue_3 2)) (and (== _returnvalue_2 2) (== _returnvalue_3 1)))
          (if (and (> _returnvalue -1) (< _returnvalue 64))
            ;[1 1 1] Check if tile is Legal
            (for _array_element_2 (`self.Out Actors`)
              (if (== (`/Game/MPChessTemplate/Blueprints/BP_Tile.TileNumber` _array_element_2) _returnvalue)
                (`|ExecutionSequence`
                  (:`then_0`
                    (break))
                  (:`then_1`
                    (if (`/Game/MPChessTemplate/Blueprints/BP_Tile.Occupied` _array_element_2)
                      (if (not (== (`/Game/MPChessTemplate/Blueprints/BP_Tile.Team` _array_element_2) (`self.Team`)))
                        (`KismetArrayLibrary.Array_Add` _validmoves _returnvalue)
                        ;[1 1 1] Check for King
                        (if (`/Game/MPChessTemplate/Blueprints/BP_Tile.King?` _array_element_2)
                          (`KismetArrayLibrary.Array_AddUnique` (`local.chktiles`) (`self.CurrentTile`))
                          (`KismetArrayLibrary.Array_AddUnique` (`local.chktiles`) _returnvalue)
                          (set `local.check?` true)
                          (set `local.Kngtile` _array_element_2)))
                      (else
                        (`KismetArrayLibrary.Array_Add` _validmoves _returnvalue))))))))))
      (:`then_1`
        (bind _returnvalue_4 (+ _currenttile _array_element))
        (bind _returnvalue_5 (`KismetMathLibrary.Abs_Int` (- (mod _returnvalue_4 8) (mod _currenttile 8))))
        (bind _returnvalue_6 (`KismetMathLibrary.Abs_Int` (- (/ _returnvalue_4 8) (/ _currenttile 8))))
        (if (or (and (== _returnvalue_5 1) (== _returnvalue_6 2)) (and (== _returnvalue_5 2) (== _returnvalue_6 1)))
          (if (and (> _returnvalue_4 -1) (< _returnvalue_4 64))
            ;[1 1 1] Check if tile is Legal
            (for _array_element_3 (`self.Out Actors`)
              (if (== (`/Game/MPChessTemplate/Blueprints/BP_Tile.TileNumber` _array_element_3) _returnvalue_4)
                (`|ExecutionSequence`
                  (:`then_0`
                    (break))
                  (:`then_1`
                    (if (`/Game/MPChessTemplate/Blueprints/BP_Tile.Occupied` _array_element_3)
                      (if (not (== (`/Game/MPChessTemplate/Blueprints/BP_Tile.Team` _array_element_3) (`self.Team`)))
                        (`KismetArrayLibrary.Array_Add` _validmoves _returnvalue_4)
                        ;[1 1 1] Check For king
                        (if (`/Game/MPChessTemplate/Blueprints/BP_Tile.King?` _array_element_3)
                          (`KismetArrayLibrary.Array_AddUnique` (`local.chktiles`) (`self.CurrentTile`))
                          (`KismetArrayLibrary.Array_AddUnique` (`local.chktiles`) _returnvalue_4)
                          (set `local.check?` true)
                          (set `local.Kngtile` _array_element_3)))
                      (else
                        (`KismetArrayLibrary.Array_Add` _validmoves _returnvalue_4))))))))))))
  (return (`self.ValidMoves`) (`local.chktiles`) (`local.check?`) (`local.Kngtile`)))

(fn `PieceMoveLogic`
  (params (Tile :type Integer) (`Occupied?` :type Boolean) (`FirstMove?` :type Boolean) (`EnemyOccupied?` :type Boolean) (`KingInCheck?` :type Boolean))
  (returns (Valid :type Boolean) (Take :type Boolean))
  (bind _currenttile (`self.CurrentTile`))
  (bind _returnvalue (`KismetMathLibrary.Abs_Int` (- (/ Tile 8) (/ _currenttile 8))))
  (bind _returnvalue_2 (`KismetMathLibrary.Abs_Int` (- (mod Tile 8) (mod _currenttile 8))))
  (if (`KismetArrayLibrary.Array_Contains` (`self.StepUnit`) (`KismetMathLibrary.Abs_Int` (- Tile (`self.CurrentTile`))))
    (if `KingInCheck?`
      (if (`KismetArrayLibrary.Array_Contains` (`self.InCheckTiles`) Tile)
        (if (or (and (== _returnvalue_2 1) (== _returnvalue 2)) (and (== _returnvalue_2 2) (== _returnvalue 1))) :!label _label
          (return true false)
          (else
            _)))
      (else
        (goto _label))))
  (return false false))

(fn `UserConstructionScript`
  (`parent.UserConstructionScript`))