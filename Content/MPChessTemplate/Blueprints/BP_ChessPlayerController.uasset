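; Player controller for a chess game that spawns the UI and camera pawn and handles one team's turn-based mouse input.
; Left click selects an own piece and spawns pointers on its valid tiles; right click sends the move through SvrMovePiece, which changes turn via the game state on success.
; Cursor box traces ignore tiles or pieces to isolate the target.
; It also drives turn, check, mate and pawn promotion UI.
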(event Custom|SvrMovePiece
  (params (Tile :type BP%20Tile%20Object%20Reference) (Piece :type BP%20Chess%20Pieces%20Object%20Reference) (Number :type Integer) (Location :type Vector))
  (bind _as_chess_game_state (Variables|Default|GetAs%20Chess%20Game%20State))
  ;[1 1 1] Controls
  (Development|PrintString (Utilities|String|Append "Attempted to move from " (Utilities|String|ToString(Integer) (Variables|/Game/MPChessTemplate/Blueprints/BP_ChessPieces.BP_ChessPieces_C|GetCurrentTile Piece)) " to " (Utilities|String|ToString(Integer) Number)) true true "(R=0.000000,G=0.660000,B=1.000000,A=1.000000)" 1e+02)
  (bind _success_ (Default|MovePiece Piece Piece Tile Number Location))
  (if _success_
    (switch int (Variables|Default|GetTeam)
      (:1
        (Default|ChangeTurn _as_chess_game_state 2))
      (:2
        (Default|ChangeTurn _as_chess_game_state 1)))
    (else
      (Development|PrintString "Failed"))))

(event Custom|PawnProm
  (params (Class :type BP%20Chess%20Pieces%20Class%20Reference) (Team :type Integer) (Tile :type Integer))
  ;[1 1 1] PawnPromotion
  (bind _asbp_chess_game_state (Utilities|Casting|CastToBP_ChessGameState (Game|GetGameState)))
  (Default|PawnPromotion _asbp_chess_game_state Class Team Tile))

(event Custom|PPZ
  ;[1 1 1] PawnPromotion
  (Widget|SetVisibility (Variables|/Game/MPChessTemplate/UI/WBP_UI.WBP_UI_C|GetPawnPromotion (Variables|UI|GetUI)) "Visible"))

(event Custom|SpawnUI
  ;[1 1 1] UI
  (Utilities|FlowControl|Sequence
    (:then_0
      (if (Pawn|IsLocalController)
        (bind _returnvalue (UserInterface|CreateWidget "/Game/MPChessTemplate/UI/WBP_UI.WBP_UI_C"))
        (UserInterface|Viewport|AddtoViewport _returnvalue 0)
        (Variables|UI|SetUI _returnvalue)))
    (:then_1
      (if (Pawn|IsLocalController)
        (bind _returnvalue_2 (UserInterface|CreateWidget "/Game/MPChessTemplate/UI/WBP_Check.WBP_Check_C"))
        (Variables|UI|SetCheckUI _returnvalue_2)))))

(event EventBeginPlay
  (Utilities|FlowControl|Sequence
    (:then_0
      (CallFunction|SpawnUI))
    (:then_1
      ;[1 1 1] Scene Setup
      (Utilities|FlowControl|Delay 1.0)
      (bind _returnvalue (Game|SpawnActorfromClass "/Game/MPChessTemplate/Blueprints/BP_CameraPawn.BP_CameraPawn_C" (Variables|Default|GetCameraTransform) "Undefined" "MultiplyWithRoot" self 0))
      (Pawn|Possess _returnvalue)
      (Development|PrintString (Utilities|String|ToString(Integer) (Variables|Default|GetTeam)) true true "(R=0.000000,G=0.660000,B=1.000000,A=1.000000)" 15.0))
    (:then_2
      (Input|SetInputModeGameandUI self 0 "DoNotLock" true false)
      (Variables|Default|SetbShowMouseCursor true))
    (:then_3
      (Utilities|FlowControl|Delay 5.0)
      (bind _asbp_chess_game_state (Utilities|Casting|CastToBP_ChessGameState (Game|GetGameState)))
      (Variables|Default|SetAs%20Chess%20Game%20State _asbp_chess_game_state))))

(event EventTick
  (params (DeltaSeconds :type Float%20%28single-precision%29)))

(event EventChangeTurn
  (params (Team :type Integer))
  ;[1 1 1] Match State
  (Default|ChangeTurn (Variables|UI|GetUI) (Variables|Default|GetMyTurn?)))

(event EventInCheckKing
  (params (NewParam :type Boolean))
  ;[1 1 1] Match State
  (bind _checkui (Variables|UI|GetCheckUI)
    (:then
      (if (Variables|Default|GetInCheck_0)
        (UserInterface|Viewport|AddtoViewport _checkui 0)
        (else
          (Widget|RemovefromParent _checkui))))
    (:else)))

(event EventPawnPromotion
  (params (Class :type BP%20Chess%20Pieces%20Class%20Reference) (Team :type Integer) (Tile :type Integer))
  ;[1 1 1] PawnPromotion
  (Widget|SetVisibility (Variables|/Game/MPChessTemplate/UI/WBP_UI.WBP_UI_C|GetPawnPromotion (Variables|UI|GetUI)) "Hidden")
  (CallFunction|PawnProm Class (Variables|Default|GetTeam) (Variables|Default|GetProPawnTile)))

(event EventPawnProZone
  (params (Tile :type Integer) (Team :type Integer))
  ;[1 1 1] PawnPromotion
  (Variables|Default|SetProPawnTile Tile)
  (CallFunction|PPZ))

(event EventMate
  (params (State :type Integer))
  (bind _ui (Variables|UI|GetUI))
  ;[1 1 1] Match State
  (Widget|SetVisibility (Variables|/Game/MPChessTemplate/UI/WBP_UI.WBP_UI_C|GetTextBlock_38 _ui) "Visible")
  (switch int State
    (:1
      (Default|PlayerStatus _ui true))
    (:2
      (Default|PlayerStatus _ui false))))

(event Input|KeyboardEvents|DebugKeyN
  (params (Key :type Key%20Structure :default "None") (ActionValue :type Input%20Action%20Value%20Structure))
  (:Pressed
    (Development|PrintString "SKIPPING TURN")
    (Default|ChangeTurn (Variables|Default|GetAs%20Chess%20Game%20State) 1)))

(event Input|MouseEvents|RightMouseButton
  (params (Key :type Key%20Structure :default "None"))
  (bind _returnvalue (Game|GetPlayerController 0))
  (bind _hitresult (Game|Player|GetHitResultUnderCursorbyChannel _returnvalue "TraceTypeQuery1" true))
  (bind _location (Collision|BreakHitResult _hitresult))
  ;[1 1 1] Controls
  (:Pressed
    (if (Variables|Default|GetMyTurn?)
      (bind _outactors (Actor|GetAllActorsOfClass "/Game/MPChessTemplate/Blueprints/BP_ChessPieces.BP_ChessPieces_C"))
      (bind _outhit (Collision|BoxTraceByChannel (+ _location "0.000000,0.000000,50.000000") (- _location "0.000000,0.000000,50.000000") "100.000000,100.000000,100.000000" "0, 0, 0" "TraceTypeQuery1" true _outactors "None"))
      (bind _asbp_tile (Utilities|Casting|CastToBP_Tile (.HitActor (Collision|BreakHitResult _outhit))))
      (bind _selectedpiece (Variables|Default|GetSelectedPiece)
        (:then
          ;;[1 1 1] Remove Pointers
          (Utilities|Array|Clear (Variables|Default|GetValid_Tiles))
          (bind _outactors_2 (Actor|GetAllActorsOfClass "/Game/MPChessTemplate/Blueprints/BP_Pointer.BP_Pointer_C"))
          (Utilities|FlowControl|Sequence
            (:then_0
              (Default|DeselectPiece (Variables|Default|GetSelectedPiece))
              (CallFunction|SvrMovePiece _asbp_tile _selectedpiece (Variables|/Game/MPChessTemplate/Blueprints/BP_Tile.BP_Tile_C|GetTileNumber _asbp_tile) (Transformation|GetActorLocation _asbp_tile))
              (Variables|Default|SetSelectedPiece 0))
            (:then_1
              (for _array_element _outactors_2
                (Actor|DestroyActor _array_element)))))
        (:else)))))

(event Input|MouseEvents|LeftMouseButton
  (params (Key :type Key%20Structure :default "None"))
  (bind _returnvalue (Game|GetPlayerController 0))
  (bind _valid_tiles (Variables|Default|GetValid_Tiles))
  (bind _hitresult (Game|Player|GetHitResultUnderCursorbyChannel _returnvalue "TraceTypeQuery1" true))
  (bind _location (Collision|BreakHitResult _hitresult))
  ;[1 1 1] Controls
  (:Pressed
    (if (Variables|Default|GetMyTurn?)
      (bind _outactors (Actor|GetAllActorsOfClass "/Game/MPChessTemplate/Blueprints/BP_ChessPieces.BP_ChessPieces_C"))
      (for _array_element _outactors
        (if (== (Variables|/Game/MPChessTemplate/Blueprints/BP_ChessPieces.BP_ChessPieces_C|GetTeam _array_element) (Variables|Default|GetTeam))
          (Default|DeselectPiece _array_element)))
      (bind _outactors_2 (Actor|GetAllActorsOfClass "/Game/MPChessTemplate/Blueprints/BP_Pointer.BP_Pointer_C"))
      (for _array_element_2 _outactors_2
        (Actor|DestroyActor _array_element_2))
      (bind _outactors_3 (Actor|GetAllActorsOfClass "/Game/MPChessTemplate/Blueprints/BP_Tile.BP_Tile_C"))
      (bind _outhit (Collision|BoxTraceByChannel (+ _location "0.000000,0.000000,50.000000") (- _location "0.000000,0.000000,50.000000") "100.000000,100.000000,100.000000" "0, 0, 0" "TraceTypeQuery1" true _outactors_3 "None"))
      (bind _asbp_chess_pieces (Utilities|Casting|CastToBP_ChessPieces (.HitActor (Collision|BreakHitResult _outhit))))
      (Development|PrintString (Utilities|GetDisplayName _asbp_chess_pieces))
      (if (== (Variables|/Game/MPChessTemplate/Blueprints/BP_ChessPieces.BP_ChessPieces_C|GetTeam _asbp_chess_pieces) (Variables|Default|GetTeam))
        (bind _output_get (Variables|Default|SetSelectedPiece _asbp_chess_pieces))
        (Default|SelectPiece _output_get)
        (Utilities|Array|Clear _valid_tiles)
        (bind _outactors_4 (Actor|GetAllActorsOfClass "/Game/MPChessTemplate/Blueprints/BP_Pointer.BP_Pointer_C"))
        (Utilities|FlowControl|Sequence
          (:then_0
            (bind _opentiles (Default|CheckAvailable _output_get _outactors_3))
            (Utilities|Array|AppendArray _valid_tiles _opentiles)
            (Utilities|FlowControl|Sequence
              (:then_0
                (bind _array_element_3 (Utilities|Array|ForEachLoopwithBreak _outactors_3)
                  (:LoopBody
                    (if (Utilities|Array|ContainsItem (Variables|Default|GetValid_Tiles) (Variables|/Game/MPChessTemplate/Blueprints/BP_Tile.BP_Tile_C|GetTileNumber _array_element_3))
                      (if (Variables|/Game/MPChessTemplate/Blueprints/BP_Tile.BP_Tile_C|GetOccupied _array_element_3)
                        (if (!= (Variables|/Game/MPChessTemplate/Blueprints/BP_Tile.BP_Tile_C|GetTeam _array_element_3) (Variables|Default|GetTeam))
                          (Game|SpawnActorfromClass "/Game/MPChessTemplate/Blueprints/BP_OccupiedPointer.BP_OccupiedPointer_C" (Math|Transform|MakeTransform (Transformation|GetActorLocation _array_element_3) "0, 0, 0" "1.000000,1.000000,1.000000") "Undefined" "MultiplyWithRoot" 0 0))
                        (else
                          (Game|SpawnActorfromClass "/Game/MPChessTemplate/Blueprints/BP_Pointer.BP_Pointer_C" (Math|Transform|MakeTransform (Transformation|GetActorLocation _array_element_3) "0, 0, 0" "1.000000,1.000000,1.000000") "Undefined" "MultiplyWithRoot" 0 0)))))))
              (:then_1
                (for _array_element_4 _opentiles
                  (Development|PrintString (Utilities|String|ToString(Integer) _array_element_4) true true "(R=1.000000,G=0.254943,B=0.000000,A=1.000000)")))))
          (:then_1
            (for _array_element_5 _outactors_4
              (Actor|DestroyActor _array_element_5))))))))

(fn ConstructionScript)

(fn CheckAvailable
  (params (Tiles :type Array%20of%20BP%20Tile%20Object%20References))
  (return 0))

(fn CheckPieceMoves
  (return 0 0 false 0 0))

(fn MovePiece
  (params (Piece :type BP%20Chess%20Pieces%20Object%20Reference) (Tile :type BP%20Tile%20Object%20Reference) (Number :type Integer) (Location :type Vector :default "0, 0, 0")))