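; Player state for the multiplayer chess template, holding a player's team, check and turn status, and win/loss tally.
; RepNotifies on InCheck and turn changes find the same-team BP_ChessPlayerController by searching all controllers, then copy the value and call its handler.
; Pawn promotion-zone and checkmate events relay to that controller the same way, while MatchConclusion increments Wins or Losses.
; The move, tile and mode functions are empty stubs.
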(event `self.ReceiveBeginPlay`)

(event `/Game/MPChessTemplate/Blueprints/BPI_ChessInterface.InCheckKing`
  (params (NewParam :type Boolean))
  (set `self.InCheck` NewParam)
  (bind _outactors (`GameplayStatics.GetAllActorsOfClass` "/Game/MPChessTemplate/Blueprints/BP_ChessPlayerController.BP_ChessPlayerController_C"))
  (for _array_element _outactors
    (if (== (`/Game/MPChessTemplate/Blueprints/BP_ChessPlayerController.Team` _array_element) (`self.Team`))
      (`|ExecutionSequence`
        (:`then_0`
          (break))
        (:`then_1`
          (set `/Game/MPChessTemplate/Blueprints/BP_ChessPlayerController.InCheck_0` (`self.InCheck`) _array_element)
          (`/Game/MPChessTemplate/Blueprints/BPI_ChessInterface.InCheckKing` _array_element false))))))

(event `/Game/MPChessTemplate/Blueprints/BPI_ChessInterface.PawnProZone`
  (params (Tile :type Integer) (Team :type Integer))
  (`self.PPZ` Tile))

(event `PPZ`
  (params (B :type Integer))
  (bind _team (`self.Team`))
  (bind _outactors (`GameplayStatics.GetAllActorsOfClass` "/Game/MPChessTemplate/Blueprints/BP_ChessPlayerController.BP_ChessPlayerController_C"))
  (for _array_element _outactors
    (if (== (`/Game/MPChessTemplate/Blueprints/BP_ChessPlayerController.Team` _array_element) _team)
      (`/Game/MPChessTemplate/Blueprints/BPI_ChessInterface.PawnProZone` _array_element B _team)
      (break))))

(event `Checkmate`
  (params (State :type Integer))
  (bind _outactors (`GameplayStatics.GetAllActorsOfClass` "/Game/MPChessTemplate/Blueprints/BP_ChessPlayerController.BP_ChessPlayerController_C"))
  (for _array_element _outactors
    (if (== (`/Game/MPChessTemplate/Blueprints/BP_ChessPlayerController.Team` _array_element) (`self.Team`))
      (`/Game/MPChessTemplate/Blueprints/BPI_ChessInterface.mate` _array_element State)
      (break))))

(event `/Game/MPChessTemplate/Blueprints/BPI_ChessInterface.mate`
  (params (State :type Integer))
  (`self.Checkmate` State))

(event `/Game/MPChessTemplate/Blueprints/BPI_ChessInterface.MatchConclusion`
  (params (WinTeam :type Integer))
  (if (== WinTeam (`self.Team`))
    (bind _result (`/Engine/EditorBlueprintResources/StandardMacros.IncrementInt` (`self.Wins`))
      (:`  `
        (set `self.Wins` _result)))
    (else
      (bind _result_2 (`/Engine/EditorBlueprintResources/StandardMacros.IncrementInt` (`self.Losses`))
        (:`  `
          (set `self.Losses` _result_2))))))

(fn `CheckAvailable`
  (params (Tiles :type "Array of /Game/MPChessTemplate/Blueprints/BP_Tile Object Reference (by ref)"))
  (returns (OpenTiles :type "Array of Integer"))
  (return))

(fn `CheckPieceMoves`
  (returns (ValidMoves :type "Array of Integer") (CheckTIles :type "Array of Integer") (`InCheck?` :type Boolean) (KingTile :type "/Game/MPChessTemplate/Blueprints/BP_Tile Object Reference") (AttackingPieces :type "Array of /Game/MPChessTemplate/Blueprints/BP_ChessPieces Object Reference"))
  (return _ _ false null))

(fn `FindTileByIndex`
  (params (Index :type Integer))
  (returns (Tile :type "/Game/MPChessTemplate/Blueprints/BP_Tile Object Reference"))
  (return null))

(fn `GetMode`
  (returns (Mode :type Integer))
  (return 0))

(fn `MovePiece`
  (params (Piece :type "/Game/MPChessTemplate/Blueprints/BP_ChessPieces Object Reference") (Tile :type "/Game/MPChessTemplate/Blueprints/BP_Tile Object Reference") (Number :type Integer) (Location :type "Vector Structure"))
  (returns (`Success?` :type Boolean))
  (return false))

(fn `OnRep_InCheck`
  (bind _outactors (`GameplayStatics.GetAllActorsOfClass` "/Game/MPChessTemplate/Blueprints/BP_ChessPlayerController.BP_ChessPlayerController_C"))
  (for _array_element _outactors
    (if (== (`/Game/MPChessTemplate/Blueprints/BP_ChessPlayerController.Team` _array_element) (`self.Team`))
      (`|ExecutionSequence`
        (:`then_0`
          (break))
        (:`then_1`
          (bind _output_get (set `/Game/MPChessTemplate/Blueprints/BP_ChessPlayerController.InCheck_0` (`self.InCheck`) _array_element))
          (`/Game/MPChessTemplate/Blueprints/BPI_ChessInterface.InCheckKing` _array_element false))))))

(fn `OnRep_MyTurn?`
  (bind _outactors (`GameplayStatics.GetAllActorsOfClass` "/Game/MPChessTemplate/Blueprints/BP_ChessPlayerController.BP_ChessPlayerController_C"))
  (for _array_element _outactors
    (if (== (`/Game/MPChessTemplate/Blueprints/BP_ChessPlayerController.Team` _array_element) (`self.Team`))
      (`|ExecutionSequence`
        (:`then_0`
          (set `/Game/MPChessTemplate/Blueprints/BP_ChessPlayerController.MyTurn?` (`self.MyTurn?`) _array_element)
          (`/Game/MPChessTemplate/Blueprints/BPI_ChessInterface.ChangeTurn` _array_element (`self.Team`)))
        (:`then_1`
          (break))))))

(fn `UserConstructionScript`)